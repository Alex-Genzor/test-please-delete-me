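; AC_CharList is an actor component that identifies which character class player 0 is using and records it as an enum.
; On BeginPlay, DefineList tries casting the player character to MiPersonajeTercera and to PersonajeInputAction in separate Sequence branches.
; A valid cast stores the typed reference and sets CharList to that class's enum value.
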(event Custom|DefineList
  (bind _returnvalue (Game|GetPlayerCharacter 0))
  (Utilities|FlowControl|Sequence
    (:then_0
      (bind _asmi_personaje_tercera (Utilities|Casting|CastToMiPersonajeTercera _returnvalue))
      (Utilities|IsValid _asmi_personaje_tercera
        (:Is%20Valid
          (Variables|Default|SetAs%20Mi%20Personaje%20Tercera _asmi_personaje_tercera)
          (Variables|Default|SetcharList "NewEnumerator1"))))
    (:then_1
      (bind _aspersonaje_input_action (Utilities|Casting|CastToPersonajeInputAction _returnvalue))
      (Utilities|IsValid _aspersonaje_input_action
        (:Is%20Valid
          (Variables|Default|SetAs%20Personaje%20Input%20Action _aspersonaje_input_action)
          (Variables|Default|SetcharList "NewEnumerator2"))))))

(event EventBeginPlay
  (CallFunction|DefineList))