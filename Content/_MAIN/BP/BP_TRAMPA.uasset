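; Single-use trap actor that damages the player character when it overlaps the DesatadorEventos trigger.
; A switch on the ACCharList CharList value picks the old-input (MiPersonajeTercera) or new-input (PersonajeInputAction) damage function.
; Each function casts the overlapping actor, subtracts Damage from VidaActual, prints the remaining health and destroys the trap.
; A failed cast leaves the trap in place.
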(event OnComponentBeginOverlap(DesatadorEventos)
  (params (OverlappedComponent :type Primitive%20Component%20Object%20Reference) (OtherActor :type Actor%20Object%20Reference) (OtherComp :type Primitive%20Component%20Object%20Reference) (OtherBodyIndex :type Integer) (bFromSweep :type Boolean) (SweepResult :type Hit%20Result%20Structure%20%28by%20ref%29))
  (switch Utilities|FlowControl|Switch|SwitchonE_EnumPlayers (Variables|/Game/_MAIN/ActorComponents/AC_CharList.AC_CharList_C|GetcharList (Variables|Default|GetAC_CharList))
    (:NewEnumerator1
      (CallFunction|RestarVidaPersonajeOLD OtherActor))
    (:NewEnumerator2
      (CallFunction|RestarVidaPersonajeNEW OtherActor))))

(fn ConstructionScript)

(fn RestarVidaPersonajeOLD
  (params (actorRef :type Actor%20Object%20Reference))
  (bind _asmi_personaje_tercera (Utilities|Casting|CastToMiPersonajeTercera actorRef))
  (bind _output_get (Variables|/Game/_MAIN/Game/MiPersonajeTercera.MiPersonajeTercera_C|SetvidaActual _asmi_personaje_tercera (- (Variables|/Game/_MAIN/Game/MiPersonajeTercera.MiPersonajeTercera_C|GetvidaActual _asmi_personaje_tercera) (Variables|Default|Getdamage))))
  (Development|PrintString (Utilities|String|ToString(Float) _output_get))
  (Actor|DestroyActor))

(fn RestarVidaPersonajeNEW
  (params (actorRef :type Actor%20Object%20Reference))
  (bind _aspersonaje_input_action (Utilities|Casting|CastToPersonajeInputAction actorRef))
  (bind _output_get (Variables|/Game/_MAIN/Game/PersonajeInputAction.PersonajeInputAction_C|SetvidaActual _aspersonaje_input_action (- (Variables|/Game/_MAIN/Game/PersonajeInputAction.PersonajeInputAction_C|GetvidaActual _aspersonaje_input_action) (Variables|Default|Getdamage))))
  (Development|PrintString (Utilities|String|ToString(Float) _output_get))
  (Actor|DestroyActor))